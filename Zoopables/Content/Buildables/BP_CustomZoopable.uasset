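; BP_CustomZoopable is a buildable stand-in that swaps itself for another buildable when play begins, apparently to make that buildable zoopable.
; On BeginPlay it spawns an actor of PassedBuildable's class at its own root transform.
; It then destroys its mesh proxy components and root component, without explicitly destroying the actor itself.
; The construction script is empty.
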(event EventBeginPlay
  (Game|SpawnActorfromClass (Utilities|GetClass (Variables|Default|GetPassedBuildable)) (Transformation|GetWorldTransform (Variables|Transformation|GetRootComponent)) "Undefined" "MultiplyWithRoot" 0 0)
  (Components|DestroyComponent (Variables|Default|GetmMeshComponentProxy))
  (Components|DestroyComponent (Variables|Default|GetBuildingMeshProxy1))
  (Components|DestroyComponent (Variables|Default|GetBuildingMeshProxy2))
  (Components|DestroyComponent (Variables|Transformation|GetRootComponent)))

(fn ConstructionScript)